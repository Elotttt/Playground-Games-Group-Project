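; Win trigger actor that ends the game when an eligible player, out of up to four, overlaps it.
; On overlap it checks player characters from index 3 down to 0 to identify the actor, then reads that player's own ValidToWin flag on BP_ThirdPersonCharacter.
; If the flag is set, it stores the player's index in PlayerWinIndex, shows Win_Widget and pauses the game.
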(event Collision|EventActorBeginOverlap
  (params (OtherActor :type Actor%20Object%20Reference))
  (bind _returnvalue (Game|GetPlayerCharacter 3))
  (bind _returnvalue_2 (Game|GetPlayerCharacter 2))
  (bind _returnvalue_3 (Game|GetPlayerCharacter 1))
  (bind _asbp_third_person_character (Utilities|Casting|CastToBP_ThirdPersonCharacter OtherActor))
  (Utilities|IsValid _returnvalue
    (:Is%20Valid
      (if (== OtherActor _returnvalue)
        (if (== (Variables|/Game/ThirdPerson/Blueprints/BP_ThirdPersonCharacter.BP_ThirdPersonCharacter_C|GetP4ValidToWin _asbp_third_person_character) true)
          (Variables|Default|SetPlayerWinIndex 3)
          (bind _returnvalue_4 (UserInterface|CreateWidget "/Game/Playground_Project/Elliots_Work/Widgets/Win_Widget.Win_Widget_C" :!label _label))
          (UserInterface|Viewport|AddtoViewport _returnvalue_4 0)
          (Game|SetGamePaused true))
        (else
          (if (== OtherActor _returnvalue_2) :!label _label_2
            (if (== (Variables|/Game/ThirdPerson/Blueprints/BP_ThirdPersonCharacter.BP_ThirdPersonCharacter_C|GetP3ValidToWin _asbp_third_person_character) true)
              (Variables|Default|SetPlayerWinIndex 2)
              (goto _label))
            (else
              (if (== OtherActor _returnvalue_3) :!label _label_3
                (if (== (Variables|/Game/ThirdPerson/Blueprints/BP_ThirdPersonCharacter.BP_ThirdPersonCharacter_C|GetP2ValidToWin _asbp_third_person_character) true)
                  (Variables|Default|SetPlayerWinIndex 1)
                  (goto _label))
                (else
                  (if (== OtherActor (Game|GetPlayerCharacter 0)) :!label _label_4
                    (if (== (Variables|/Game/ThirdPerson/Blueprints/BP_ThirdPersonCharacter.BP_ThirdPersonCharacter_C|GetP1ValidToWin _asbp_third_person_character) true)
                      (Variables|Default|SetPlayerWinIndex 0)
                      (goto _label))))))))))
    (:Is%20Not%20Valid
      (Utilities|IsValid _returnvalue_2
        (:Is%20Valid
          (goto _label_2))
        (:Is%20Not%20Valid
          (Utilities|IsValid _returnvalue_3
            (:Is%20Valid
              (goto _label_3))
            (:Is%20Not%20Valid
              (goto _label_4))))))))

(fn ConstructionScript)