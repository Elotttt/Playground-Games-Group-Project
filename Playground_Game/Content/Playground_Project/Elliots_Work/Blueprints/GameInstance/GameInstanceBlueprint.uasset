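; Game instance Blueprint that manages the loading screen and main menu widgets and loads saved game data.
; ShowMainMenu removes an existing menu or creates and displays one.
; CreateLoadingScreen replaces the widget only when one already exists, without adding the new one to the viewport.
; LoadGame reads slot "1", casts it to SaveBlueprint and copies its data into SaveData, printing a message when no save exists.
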(event Custom|RemoveLoadingScreen
  (bind _myloadingscreen (Variables|Default|GetMyLoadingScreen)
    (:then
      (Widget|RemovefromParent _myloadingscreen))
    (:else)))

(event Custom|CreateLoadingScreen
  (bind _myloadingscreen (Variables|Default|GetMyLoadingScreen)
    (:then
      (Widget|RemovefromParent _myloadingscreen)
      (bind _returnvalue (UserInterface|CreateWidget "/Game/Playground_Project/Elliots_Work/Widgets/LoadingScreen.LoadingScreen_C" (Game|GetPlayerController 0)))
      (Variables|Default|SetMyLoadingScreen _returnvalue))
    (:else)))

(event Custom|ShowMainMenu
  (bind _mymainmenu (Variables|Default|GetMyMainMenu)
    (:then
      (Widget|RemovefromParent _mymainmenu))
    (:else
      (bind _returnvalue (UserInterface|CreateWidget "/Game/Playground_Project/Elliots_Work/Widgets/MenuWidget.MenuWidget_C" (Game|GetPlayerController 0)))
      (Variables|Default|SetMyMainMenu _returnvalue)
      (UserInterface|Viewport|AddtoViewport _returnvalue 0))))

(event Custom|LoadGame
  (bind _returnvalue (SaveGame|DoesSaveGameExist "1"))
  (if _returnvalue
    (bind _returnvalue_2 (SaveGame|LoadGamefromSlot "1"))
    (Variables|Default|SetSaveData (Variables|/Game/Playground_Project/Elliots_Work/Blueprints/GameInstance/SaveBlueprint.SaveBlueprint_C|GetMySaveData (.AsSave%20Blueprint (Utilities|Casting|CastToSaveBlueprint _returnvalue_2))))
    (else
      (Development|PrintString "Failed to load save"))))